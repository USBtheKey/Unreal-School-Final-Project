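; Turret actor that tracks the first-person player and fires projectiles when the player is within range.
; BeginPlay caches the player character, and Tick runs a distance check that also switches the range indicator between red and green materials.
; While in range, it snaps yaw-only toward the player and spawns TurretProjectileBP at BulletSpawnPoint.
; A DoOnce reset after a Delay limits fire to about one shot per second.
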(event EventBeginPlay
  (bind _asfirst_person_character (Utilities|Casting|CastToFirstPersonCharacter (Game|GetPlayerCharacter 0)))
  (Variables|Default|SetfirstPersonCharacter _asfirst_person_character))

(event EventTick
  (params (DeltaSeconds :type Float%20%28single-precision%29))
  (bind _islessthan_excluded_1000_ (CallFunction|CheckDistance))
  (if _islessthan_excluded_1000_
    (CallFunction|LookatPlayer)
    (Utilities|FlowControl|DoOnce false :!label _label
      (:Completed
        (Game|SpawnActorfromClass "/Game/TurretProjectileBP.TurretProjectileBP_C" (Transformation|GetWorldTransform (Variables|Default|GetbulletSpawnPoint)) "Undefined" 0 0)
        (Utilities|FlowControl|Delay 1.0)
        (goto _label Reset)))))

(fn ConstructionScript)

(fn LookatPlayer
  (Transformation|SetActorRotation (Math|Rotator|MakeRotator 0.0 0.0 (.Yaw (Math|Rotator|BreakRotator (Math|Rotator|FindLookatRotation (Transformation|GetActorLocation) (Transformation|GetActorLocation (Variables|Default|GetfirstPersonCharacter))))))))

(fn CheckDistance
  (bind _returnvalue (Transformation|GetActorLocation))
  (bind _firstpersoncharacter (Variables|Default|GetfirstPersonCharacter))
  (bind _returnvalue_2 (Transformation|GetActorLocation _firstpersoncharacter))
  (bind _returnvalue_3 (- _returnvalue_2 _returnvalue))
  (bind _returnvalue_4 (Math|Vector|VectorLength _returnvalue_3))
  (bind _returnvalue_5 (< _returnvalue_4 1e+03))
  (if _returnvalue_5
    (Rendering|Material|SetMaterial (Variables|Default|GetTargetInRange) 0 "/Game/LightRed.LightRed")
    (else
      (Rendering|Material|SetMaterial (Variables|Default|GetTargetInRange) 0 "/Game/LightGreen.LightGreen")))
  (return _returnvalue_5))